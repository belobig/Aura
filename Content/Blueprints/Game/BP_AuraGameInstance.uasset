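; Game instance Blueprint that manages main menu music and shows a map change screen.
; Music events spawn a 2D sound that persists across level transitions, store it, and fade or stop it while tracking a MusicOn flag.
; OnMapChange creates a WBP_MapChange widget, fills its level name from the Aura game mode's map asset name lookup, and adds it to the viewport.
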(event Custom|PlayMainMenuMusic
  (params (Sound :type Sound%20Base%20Object%20Reference))
  (bind _returnvalue (Audio|SpawnSound2D Sound 1.0 1.0 0.0 0 true))
  (Variables|Default|SetMainMenuMusic _returnvalue)
  (Variables|Default|SetMusicOn true))

(event Custom|StopMainMenuMusic
  (Utilities|IsValid (Variables|Default|GetMainMenuMusic)
    (:Is%20Valid
      (Audio|Components|Audio|Stop (Variables|Default|GetMainMenuMusic))
      (Variables|Default|SetMusicOn false))))

(event Custom|FadeMainMenuMusic
  (Utilities|IsValid (Variables|Default|GetMainMenuMusic)
    (:Is%20Valid
      (Audio|Components|Audio|FadeOut (Variables|Default|GetMainMenuMusic) (Variables|Default|GetFadeOutDuration) 0.0 "Linear" :!class /Script/Engine.AudioComponent)
      (Variables|Default|SetMusicOn false))))

(event Custom|OnMapChange
  (CallFunction|DisplayMapChangeWidget))

(fn DisplayMapChangeWidget
  (bind _returnvalue (UserInterface|CreateWidget "/Game/Blueprints/UI/MapChange/WBP_MapChange.WBP_MapChange_C"))
  (bind _asaura_game_mode_base (Utilities|Casting|CastToAuraGameModeBase (Game|GetGameMode)))
  (bind _returnvalue_2 (Game|GetCurrentLevelName true))
  (Variables|/Game/Blueprints/UI/MapChange/WBP_MapChange.WBP_MapChange_C|SetInLevelName _returnvalue (Utilities|Text|ToText(String) (Class|AuraGameModeBase|GetMapNamefromMapAssetName _asaura_game_mode_base _returnvalue_2)))
  (UserInterface|Viewport|AddtoViewport _returnvalue 0))