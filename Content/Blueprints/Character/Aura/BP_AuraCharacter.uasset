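; Player character Blueprint for Aura, adding facing, shock-loop state and overlap-driven message fading.
; Interface-style events feed a FacingTarget location to Motion Warping and set the InShockLoop flag.
; A Box overlap fades the other actor's message out on entry and back in on exit, only while locally controlled and moving.
; Falling out of the world only prints a debug string, depending on whether a game mode is valid.
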(event OnComponentBeginOverlap(Box)
  (params (OverlappedComponent :type Primitive%20Component%20Object%20Reference) (OtherActor :type Actor%20Object%20Reference) (OtherComp :type Primitive%20Component%20Object%20Reference) (OtherBodyIndex :type Integer) (bFromSweep :type Boolean) (SweepResult :type Hit%20Result%20Structure%20%28by%20ref%29))
  (if (Pawn|IsLocallyControlled)
    (bind _returnvalue (CallFunction|IsMoving))
    (if _returnvalue
      (Class|BIFadeInterface|FadeOut(Message) OtherActor))))

(event OnComponentEndOverlap(Box)
  (params (OverlappedComponent :type Primitive%20Component%20Object%20Reference) (OtherActor :type Actor%20Object%20Reference) (OtherComp :type Primitive%20Component%20Object%20Reference) (OtherBodyIndex :type Integer))
  (if (Pawn|IsLocallyControlled)
    (bind _returnvalue (CallFunction|IsMoving))
    (if _returnvalue
      (Class|BIFadeInterface|Fadein(Message) OtherActor))))

(event EventSetinShockLoop
  (params (bInLoop :type Boolean))
  (Variables|Default|SetInShockLoop bInLoop))

(event EventOnFellOutOfWorld
  (Utilities|IsValid (Game|GetGameMode)
    (:Is%20Valid
      (Development|PrintString "You fell out of the world" true true "(R=1.000000,G=0.336096,B=0.001209,A=1.000000)"))
    (:Is%20Not%20Valid
      (Development|PrintString "No valid game mode" true true "(R=1.000000,G=0.000000,B=0.000333,A=1.000000)"))))

(event EventUpdateFacingTarget
  (params (Target :type Vector%20%28by%20ref%29 :default "0, 0, 0"))
  (Class|MotionWarpingComponent|AddorUpdateWarpTargetfromLocation (Variables|Default|GetMotionWarping) "FacingTarget" Target))

(fn ConstructionScript)

(fn IsMoving
  (return (> (Math|Vector|VectorLength (Variables|/Script/Engine.MovementComponent|GetVelocity (Variables|Character|GetCharacterMovement))) 0.0)))